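; Game state Blueprint for a turn-based game, holding a helper function that spawns actors by name on the current player's side.
; TheVeryStupidStuff reads CurrentPlayer from the game state to pick one of two mirrored spawn positions on the X axis.
; It then matches the given name against hardcoded strings to spawn either BP_Territory or BP_TheFirst.
; The event graph and construction script are empty.
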(fn `TheVeryStupidStuff`
  (params (Name :type Text))
  (locals (CurrentName :type Text) (SpawnTransform :type "Transform Structure"))
  (bind _spawntransform (`local.SpawnTransform`))
  (bind _asbp_turn_based_game_state (cast `/Game/MyStuff/TurnBased/BP_TurnBasedGameState` (`GameplayStatics.GetGameState`)))
  (if (== (`/Game/MyStuff/TurnBased/BP_TurnBasedGameState.CurrentPlayer` _asbp_turn_based_game_state) 0)
    (set `local.SpawnTransform` (`KismetMathLibrary.MakeTransform` (15.0 0.0 0.0)))
    (else
      (set `local.SpawnTransform` (`KismetMathLibrary.MakeTransform` (-15.0 0.0 0.0)))))
  (bind _output_get (set `local.CurrentName` "territory"))
  (if (== _output_get Name)
    (`|SpawnActorFromClass` "/Game/MyStuff/PhysicalCards/BP_Territory.BP_Territory_C" _spawntransform "Undefined" "MultiplyWithRoot" null null)
    (else
      (bind _output_get_2 (set `local.CurrentName` "the first"))
      (if (== _output_get_2 Name)
        (`|SpawnActorFromClass` "/Game/MyStuff/PhysicalCards/BP_TheFirst.BP_TheFirst_C" _spawntransform "Undefined" "MultiplyWithRoot" null null)))))

(fn `UserConstructionScript`)