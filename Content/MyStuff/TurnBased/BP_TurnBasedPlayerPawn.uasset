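; BP_TurnBasedPlayerPawn is the player pawn that acts as a movable camera, named for turn-based play.
; MoveX, MoveY and MoveZ axes drive movement input along actor forward, actor right and world up, scaled by CameraSpeed.
; Holding the right mouse button sets RightDown, which lets mouse X and Y feed controller yaw and negated pitch.
; It contains no turn logic, only movement and look input.
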(event `InputAxis|MoveX`
  (params (AxisValue :type "Float (single-precision)"))
  (`self.AddMovementInput` (`self.GetActorForwardVector`) (* AxisValue (`self.CameraSpeed`))))

(event `InputAxis|MoveY`
  (params (AxisValue :type "Float (single-precision)"))
  (`self.AddMovementInput` (`self.GetActorRightVector`) (* AxisValue (`self.CameraSpeed`))))

(event `InputAxis|MoveZ`
  (params (AxisValue :type "Float (single-precision)"))
  (`self.AddMovementInput` (`KismetMathLibrary.Vector_Up`) (* AxisValue (`self.CameraSpeed`))))

(event `Key|RightMouseButton`
  (params (Key :type "Key Structure"))
  (:`Pressed`
    (set `self.RightDown` true))
  (:`Released`
    (set `self.RightDown` false)))

(event `InputAxisKey|MouseX`
  (params (AxisValue :type "Float (single-precision)"))
  (if (`self.RightDown`)
    (`self.AddControllerYawInput` AxisValue)))

(event `InputAxisKey|MouseY`
  (params (AxisValue :type "Float (single-precision)"))
  (if (`self.RightDown`)
    (`self.AddControllerPitchInput` (* AxisValue -1.0))))

(fn `UserConstructionScript`)