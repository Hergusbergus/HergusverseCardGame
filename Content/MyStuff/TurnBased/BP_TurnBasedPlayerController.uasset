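; BP_TurnBasedPlayerController is the player controller for a turn-based game, tracking whether it is this player's turn.
; On BeginPlay, the local controller creates WB_MainUI and adds it to the viewport.
; StartTurn and EndTurn update MyTurn through SetMyTurn, which fires OnMyTurnChange with the new value.
; PassTurn and PassPhase forward to BP_TurnBasedGameMode to cycle the turn or phase.
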(event `self.ReceiveBeginPlay`
  (if (`self.IsLocalController`)
    (bind _returnvalue (`|CreateWidget` "/Game/MyStuff/UI/WB_MainUI.WB_MainUI_C" self))
    (`UserWidget.AddToViewport` _returnvalue 0)))

(event `Start Turn`
  (`self.SetMyTurn` true))

(event `End Turn`
  (`self.SetMyTurn` false))

(event `Pass Turn`
  (bind _asbp_turn_based_game_mode (cast `/Game/MyStuff/TurnBased/BP_TurnBasedGameMode` (`GameplayStatics.GetGameMode`)))
  (`/Game/MyStuff/TurnBased/BP_TurnBasedGameMode.Cycle Turn` _asbp_turn_based_game_mode))

(event `Pass Phase`
  (bind _asbp_turn_based_game_mode (cast `/Game/MyStuff/TurnBased/BP_TurnBasedGameMode` (`GameplayStatics.GetGameMode`)))
  (`/Game/MyStuff/TurnBased/BP_TurnBasedGameMode.Cycle Phase` _asbp_turn_based_game_mode))

(fn `SetMyTurn`
  (params (MyTurn :type Boolean))
  (bind _output_get (set `self.MyTurn` MyTurn))
  (`self.OnMyTurnChange` _output_get))

(fn `UserConstructionScript`)